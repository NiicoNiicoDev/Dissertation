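; VR shop actor where the player sells owned weapons or buys the shopkeeper's by grabbing offered coins.
; A collider captures items with WeaponData, and Tick waits for release before snapping them to the display spot once.
; Timed merchant widget dialogue quotes the price while coins appear.
; Grabbing adjusts VRPawn coins: sales pay 80% of price and destroy the item, while purchases deduct full price without a balance check and relocate it.
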(event `self.ReceiveBeginPlay`)

(event `self.ReceiveTick`
  (params (DeltaSeconds :type "Float (single-precision)"))
  (bind _returnvalue (`self.GetComponentByClass` (`self.Other Actor`) "/Script/Engine.StaticMeshComponent"))
  (if (`PrimitiveComponent.IsOverlappingActor` (`self.  ShopCollider`) (`self.Other Actor`))
    (if (not (`/Game/VRTemplate/Blueprints/GrabComponent.bIsHeld` (`self.GetComponentByClass` (`self.Other Actor`) "/Game/VRTemplate/Blueprints/GrabComponent.GrabComponent_C")))
      (`/Engine/EditorBlueprintResources/StandardMacros.DoOnce` false :!label _label
        (:`Completed`
          (`PrimitiveComponent.SetPhysicsLinearVelocity` _returnvalue (0.0 0.0 0.0) false "None")
          (`PrimitiveComponent.SetPhysicsAngularVelocityInDegrees` _returnvalue (0.0 0.0 0.0) false "None")
          (if (`/Game/Weapons/Blueprints/WeaponData.isPlayerOwned` (`self.WeaponData`))
            (`|ExecutionSequence`
              (:`then_0`
                (`SceneComponent.SetVisibility` (`self.coins`) true false)
                (`self.K2_SetActorTransform` (`self.Other Actor`) (`SceneComponent.K2_GetComponentToWorld` (`self.ItemLocation`)) false false))
              (:`then_1`
                (`self.SetShopTextInactive` "Visible")
                (`self.ShowItemPrice` "Ooh an interesting item I see, I'd be interested in buying this one from you")
                (`KismetSystemLibrary.Delay` 5.0)
                (`self.ShowItemPrice` "Hmm.. Let me just think up a price")
                (`KismetSystemLibrary.Delay` 5.0)
                (`/Engine/EditorBlueprintResources/StandardMacros.IsValid` (`self.WeaponData`)
                  (:`Is Valid`
                    (`self.ShowItemPrice` (`KismetTextLibrary.Conv_StringToText` (`KismetStringLibrary.Concat_StrStr` (`KismetStringLibrary.Concat_StrStr` "I think i will offer you " (`KismetStringLibrary.Conv_IntToString` (`/Game/Weapons/Blueprints/WeaponData.Price` (`self.WeaponData`)))) " coin")))
                    (`KismetSystemLibrary.Delay` 5.0)
                    (`self.ShowItemPrice` "I've popped some coins over on the left, grab them to accept my offer"))
                  (:`Is Not Valid`
                    (`self.ShowItemPrice` "Oh the weapon seems to either not be in the correct place or seems to have vanished? What kind of wizardry is this?!?")))))
            (else
              (`|ExecutionSequence`
                (:`then_0`
                  (`self.SetShopTextInactive` "Visible")
                  (`self.ShowItemPrice` "It's a good weapon that one is, ")
                  (`KismetSystemLibrary.Delay` 5.0)
                  (`self.ShowItemPrice` "I'd only sell it if the price was right...")
                  (`KismetSystemLibrary.Delay` 5.0)
                  (`/Engine/EditorBlueprintResources/StandardMacros.IsValid` (`self.WeaponData`)
                    (:`Is Valid`
                      (`self.ShowItemPrice` (`KismetTextLibrary.Conv_StringToText` (`KismetStringLibrary.Concat_StrStr` (`KismetStringLibrary.Concat_StrStr` "I don't know let's say " (`KismetStringLibrary.Conv_IntToString` (`/Game/Weapons/Blueprints/WeaponData.Price` (`self.WeaponData`)))) " coin")))
                      (`KismetSystemLibrary.Delay` 3.0)
                      (`self.ShowItemPrice` "I've popped some coins over on the left, grab them to buy the item from me")
                      (`KismetSystemLibrary.Delay` 3.0)
                      (`self.ShowItemPrice` "Once you've bought the item, i'll pop it on the item stand just to your right you so you can pick it up"))))
                (:`then_1`
                  (`SceneComponent.SetVisibility` (`self.coins`) true false)
                  (`self.K2_SetActorTransform` (`self.Other Actor`) (`SceneComponent.K2_GetComponentToWorld` (`self.ItemLocation`)) false false))))))))))

(event `self.  ShopCollider.OnComponentEndOverlap`
  (params (OverlappedComponent :type "PrimitiveComponent Object Reference") (OtherActor :type "Actor Object Reference") (OtherComp :type "PrimitiveComponent Object Reference") (OtherBodyIndex :type Integer))
  (if (== (`self.Other Actor`) OtherActor)
    (`SceneComponent.SetVisibility` (`self.coins`) false false)
    (`self.SetShopTextInactive` "Hidden")
    (set `self.Other Actor` null)
    (set `self.WeaponData` null)
    (goto _label :!via `Reset`)))

(event `self.  ShopCollider.OnComponentBeginOverlap`
  (params (OverlappedComponent :type "PrimitiveComponent Object Reference") (OtherActor :type "Actor Object Reference") (OtherComp :type "PrimitiveComponent Object Reference") (OtherBodyIndex :type Integer) (bFromSweep :type Boolean) (SweepResult :type "HitResult Structure (by ref)"))
  (bind _returnvalue (`self.GetComponentByClass` OtherActor "/Game/Weapons/Blueprints/WeaponData.WeaponData_C"))
  (`/Engine/EditorBlueprintResources/StandardMacros.IsValid` _returnvalue
    (:`Is Valid`
      (set `self.Other Actor` OtherActor)
      (set `self.WeaponData` _returnvalue))))

(event `self.GrabComponent.OnGrabbed`
  (if (`/Game/Weapons/Blueprints/WeaponData.isPlayerOwned` (`self.WeaponData`))
    (`SceneComponent.SetVisibility` (`self.coins`) false false)
    (bind _returnvalue (`GameplayStatics.GetActorOfClass` "/Game/VRTemplate/Blueprints/VRPawn.VRPawn_C"))
    (set `/Game/VRTemplate/Blueprints/VRPawn.Coins` (+ (`/Game/VRTemplate/Blueprints/VRPawn.Coins` _returnvalue) (* (`/Game/Weapons/Blueprints/WeaponData.Price` (`self.WeaponData`)) 0.8)) _returnvalue)
    (`self.K2_DestroyActor` (`self.Other Actor`))
    (set `self.Other Actor` null)
    (set `self.WeaponData` null)
    (goto _label :!via `Reset`)
    (else
      (`SceneComponent.SetVisibility` (`self.coins`) false false)
      (bind _returnvalue_2 (`GameplayStatics.GetActorOfClass` "/Game/VRTemplate/Blueprints/VRPawn.VRPawn_C"))
      (set `/Game/VRTemplate/Blueprints/VRPawn.Coins` (- (`/Game/VRTemplate/Blueprints/VRPawn.Coins` _returnvalue_2) (`/Game/Weapons/Blueprints/WeaponData.Price` (`self.WeaponData`))) _returnvalue_2)
      (set `/Game/Weapons/Blueprints/WeaponData.isPlayerOwned` true (`self.WeaponData`))
      (`self.K2_SetActorTransform` (`self.Other Actor`) (`self.BuyTransform`) false false)
      (set `self.Other Actor` null)
      (set `self.WeaponData` null)
      (goto _label :!via `Reset`))))

(fn `SetShopTextInactive`
  (params (Visiblity :type "ESlateVisibility Enum" :default "Visible"))
  (`Widget.SetVisibility` (`WidgetComponent.GetWidget` (`self.ShopKeeperTextActor`)) Visiblity))

(fn `ShowItemPrice`
  (params (ShopKeeperText :type Text))
  (bind _aswbp_merchant_text (cast `/Game/Shop/WBP_MerchantText` (`WidgetComponent.GetWidget` (`self.ShopKeeperTextActor`))))
  (set `MultiLineEditableTextBox.Text` ShopKeeperText (`/Game/Shop/WBP_MerchantText.Text` _aswbp_merchant_text)))

(fn `UserConstructionScript`)