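; Weapon Blueprint for a physics-driven weapon that snaps back to its spawn point if an unowned copy is moved too far away.
; BeginPlay caches the shop actor and the weapon's starting transform.
; While the shop reference is valid and the player does not own the weapon, Tick checks its distance from spawn.
; Past the threshold, it teleports back and zeroes the mesh's linear and angular physics velocity.
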(event `self.ReceiveBeginPlay`
  (bind _returnvalue (`GameplayStatics.GetActorOfClass` "/Game/Shop/BP_ShopActor.BP_ShopActor_C"))
  (set `self.ShopActor` _returnvalue)
  (set `self.SpawnTransform` (`self.GetTransform`)))

(event `self.ReceiveActorBeginOverlap`
  (params (OtherActor :type "Actor Object Reference")))

(event `self.ReceiveTick`
  (params (DeltaSeconds :type "Float (single-precision)"))
  (bind _returnvalue_location (`KismetMathLibrary.BreakTransform` (`self.GetTransform`)))
  (bind _spawntransform_location (`KismetMathLibrary.BreakTransform` (`self.SpawnTransform`)))
  (`/Engine/EditorBlueprintResources/StandardMacros.IsValid` (`self.ShopActor`)
    (:`Is Valid`
      (if (`/Game/Weapons/Blueprints/WeaponData.isPlayerOwned` (`self.WeaponData`))
        _
        (elif (>= (`KismetMathLibrary.Vector_Distance` _returnvalue_location _spawntransform_location) 750.0)
          (`self.K2_SetActorTransform` (`self.SpawnTransform`) false true)
          (`PrimitiveComponent.SetPhysicsLinearVelocity` (`self.StaticMeshComponent`) (0.0 0.0 0.0) false "None")
          (`PrimitiveComponent.SetPhysicsAngularVelocityInDegrees` (`self.StaticMeshComponent`) (0.0 0.0 0.0) false "None"))))))

(fn `UserConstructionScript`)