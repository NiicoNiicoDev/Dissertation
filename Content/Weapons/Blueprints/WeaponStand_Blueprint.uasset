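; Weapon stand that displays a placed weapon with its name, damage and level requirement on a widget.
; Box overlap captures one actor with a WeaponData component, fills the widget and registers it as InventoryPlaceable's stored item.
; Tick waits until its GrabComponent is released, then attaches it to the stand and eases it via Timeline to that weapon's stand transform.
; Ending overlap clears the widget and stored references.
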(event `self.ReceiveBeginPlay`)

(event `self.Box.OnComponentBeginOverlap`
  (params (OverlappedComponent :type "PrimitiveComponent Object Reference") (OtherActor :type "Actor Object Reference") (OtherComp :type "PrimitiveComponent Object Reference") (OtherBodyIndex :type Integer) (bFromSweep :type Boolean) (SweepResult :type "HitResult Structure (by ref)"))
  (if (not (`self.isPlaced`))
    (`/Engine/EditorBlueprintResources/StandardMacros.IsValid` (`self.WeaponActor`)
      (:`Is Not Valid`
        (bind _returnvalue (`MyBlueprintFunctionLibrary.DoesActorContainClass` OtherActor "/Game/Weapons/Blueprints/WeaponData.WeaponData_C"))
        (if _returnvalue
          (set `self.WeaponActor` OtherActor)
          (set `self.Weapon Data` (`self.GetComponentByClass` OtherActor "/Game/Weapons/Blueprints/WeaponData.WeaponData_C"))
          (bind _asweapon_stand_widget (cast `/Game/Weapons/UI/WeaponStand/WeaponStandWidget` (`WidgetComponent.GetWidget` (`self.Widget`))))
          (set `self.Weapon Stand Widget` _asweapon_stand_widget)
          (set `self.IsWeaponInOverlap` true)
          (`self.SetData` (`self.Weapon Data`) (`self.Weapon Stand Widget`))
          (set `InventoryPlaceable.storedItem` (`self.WeaponActor`) (`self.InventoryPlaceable`)))))))

(event `self.Box.OnComponentEndOverlap`
  (params (OverlappedComponent :type "PrimitiveComponent Object Reference") (OtherActor :type "Actor Object Reference") (OtherComp :type "PrimitiveComponent Object Reference") (OtherBodyIndex :type Integer))
  (if (== OtherActor (`self.WeaponActor`))
    (set `self.IsWeaponInOverlap` false)
    (`self.SetData` (`self.Weapon Data`) (`self.Weapon Stand Widget`) true)
    (set `self.isPlaced` false)
    (`self.K2_DetachFromActor` "KeepWorld" "KeepWorld" "KeepWorld")
    (set `self.WeaponActor` null)
    (set `self.Weapon Data` null)
    (set `InventoryPlaceable.storedItem` null (`self.InventoryPlaceable`))))

(event `self.ReceiveTick`
  (params (DeltaSeconds :type "Float (single-precision)"))
  (bind _weapon_data (`self.Weapon Data`))
  (bind _rootcomponent (`Actor.RootComponent` (`self.WeaponActor`)))
  (if (`self.IsWeaponInOverlap`)
    (if (`/Game/VRTemplate/Blueprints/GrabComponent.bIsHeld` (`self.GetComponentByClass` (`self.WeaponActor`) "/Game/VRTemplate/Blueprints/GrabComponent.GrabComponent_C"))
      _
      (elif (not (`self.isPlaced`))
        (set `self.isPlaced` true)
        (`self.Set Object Parent` (`self.WeaponActor`))
        (bind (_direction _newtrack_0) (`Timeline|Timeline` :!via `PlayFromStart` :!label _label)
          (:`Update`
            (`SceneComponent.K2_SetRelativeTransform` _rootcomponent (`KismetMathLibrary.TLerp` (`SceneComponent.GetRelativeTransform` _rootcomponent) (`KismetMathLibrary.MakeTransform` (`/Game/Weapons/Blueprints/WeaponData.StandPos` _weapon_data) (`/Game/Weapons/Blueprints/WeaponData.StandRotation` _weapon_data)) _newtrack_0) false false))
          (:`Finished`
            (goto _label :!via `Stop`)))))))

(fn `Set Object Parent`
  (params (Weapon :type "Actor Object Reference"))
  (`self.K2_AttachToActor` Weapon self "None" "KeepWorld" "KeepWorld" "KeepWorld" true))

(fn `Set Object Position And Rotation`
  (params (DeltaTime :type "Float (double-precision)") (`Start Transform` :type "Transform Structure") (`End Transform` :type "Transform Structure") (WeaponActor :type "Actor Object Reference"))
  (locals (NewLocalVar :type "Transform Structure")))

(fn `SetData`
  (params (WeaponData :type "/Game/Weapons/Blueprints/WeaponData Object Reference") (WeaponStandWidget :type "/Game/Weapons/UI/WeaponStand/WeaponStandWidget Object Reference") (ResetData :type Boolean))
  (bind _itemname (`/Game/Weapons/UI/WeaponStand/WeaponStandWidget.ItemName` WeaponStandWidget))
  (bind _itemdamage (`/Game/Weapons/UI/WeaponStand/WeaponStandWidget.ItemDamage` WeaponStandWidget))
  (bind _itemlevel (`/Game/Weapons/UI/WeaponStand/WeaponStandWidget.ItemLevel` WeaponStandWidget))
  (if ResetData
    (`TextBlock.SetText` _itemname "")
    (`TextBlock.SetText` _itemdamage "")
    (`TextBlock.SetText` _itemlevel "")
    (else
      (`TextBlock.SetText` _itemname (`KismetTextLibrary.Conv_StringToText` (`/Game/Weapons/Blueprints/WeaponData.Name` WeaponData)))
      (`TextBlock.SetText` _itemdamage (`KismetTextLibrary.Conv_IntToText` (`/Game/Weapons/Blueprints/WeaponData.Damage` WeaponData)))
      (`TextBlock.SetText` _itemlevel (`KismetTextLibrary.Conv_Int64ToText` (`/Game/Weapons/Blueprints/WeaponData.Level Requirement` WeaponData))))))

(fn `UserConstructionScript`)